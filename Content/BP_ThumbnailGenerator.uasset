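; Thumbnail generator actor that batch-exports TGA images of static meshes and materials.
; CaptureAll picks a mode (models, materials, all, debug or a specified index), swaps the mesh, scales it to fit a reference bound and applies each material.
; A SceneCapture2D matched to the camera renders to RT and exports files named from mesh and material.
; Construction derives the save folder from RT's location, falling back to Saved/ThumbnailHelper; the alpha-mask pass is disconnected.
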(fn `AlphaMaskSetup`
  (params (AlphaMask :type Boolean))
  (bind _backgroundmat (`self.BackgroundMat`))
  (bind _alphazeromat (`self.AlphaZeroMat`))
  (if AlphaMask
    (`PrimitiveComponent.SetMaterial` (`self.NeedCaptureObject`) 0 (`self.AlphaOneMat`))
    (`PrimitiveComponent.SetMaterial` (`self.Background1`) 0 _alphazeromat)
    (`PrimitiveComponent.SetMaterial` (`self.Background`) 0 _alphazeromat)
    (else
      (`PrimitiveComponent.SetMaterial` (`self.Background`) 0 _backgroundmat)
      (`PrimitiveComponent.SetMaterial` (`self.Background1`) 0 _backgroundmat))))

(fn `Capture Mat Thumbnails`
  (params (TargetMats :type "Array of MaterialInstanceConstant Object Reference (by ref)"))
  (bind _prefix_log (`self.Prefix-Log`))
  (bind _needcaptureobject (`self.NeedCaptureObject`))
  (if (> (`KismetArrayLibrary.Array_Length` TargetMats) 0)
    (`KismetSystemLibrary.PrintString` (`KismetStringLibrary.Concat_StrStr` _prefix_log "开始生成材质缩略图"))
    (for _array_element TargetMats
      (`PrimitiveComponent.SetMaterial` _needcaptureobject 0 _array_element)
      (`self.AlphaMaskSetup` false)
      (`self.ExportThumbnail` (`KismetStringLibrary.Concat_StrStr` "T_Thumb_" (`KismetStringLibrary.Concat_StrStr` (`.RightS` (`KismetStringLibrary.Split` (`KismetSystemLibrary.GetDisplayName` (`StaticMeshComponent.StaticMesh` _needcaptureobject)) "_")) "_" (`.RightS` (`KismetStringLibrary.Split` (`KismetSystemLibrary.GetDisplayName` _array_element) "_"))) "_RGB")))
    (else
      (`KismetSystemLibrary.PrintString` (`KismetStringLibrary.Concat_StrStr` _prefix_log "没有要生成的材质！")))))

(fn `Capture Mesh Original Thumbnails`
  (bind _meshs (`self.Meshs`))
  (bind _prefix_log (`self.Prefix-Log`))
  (if (> (`KismetArrayLibrary.Array_Length` _meshs) 0)
    (`KismetSystemLibrary.PrintString` (`KismetStringLibrary.Concat_StrStr` _prefix_log "开始生成模型默认材质缩略图"))
    (for _array_element _meshs
      (bind _res (`self.UpdateNeedCaptureMesh` _array_element))
      (if _res
        (`self.Capture Mat Thumbnails` (`|MakeArray` (`self.DefaultMat`)))))
    (else
      (`KismetSystemLibrary.PrintString` (`KismetStringLibrary.Concat_StrStr` _prefix_log "没有要生成的模型！")))))

(fn `Capture SpecifiedMesh Thumbnails`
  (params (TargetMats :type "Array of MaterialInstanceConstant Object Reference (by ref)") (InputObject :type "StaticMesh Object Reference"))
  (bind _prefix_log (`self.Prefix-Log`))
  (`/Engine/EditorBlueprintResources/StandardMacros.IsValid` InputObject
    (:`Is Valid`
      (if (> (`KismetArrayLibrary.Array_Length` TargetMats) 0)
        (`KismetSystemLibrary.PrintString` (`KismetStringLibrary.Concat_StrStr` _prefix_log "开始生成模型缩略图"))
        (bind _res (`self.UpdateNeedCaptureMesh` InputObject))
        (if _res
          (`self.Capture Mat Thumbnails` TargetMats)
          (else
            (`self.FailLog` "Function  [CaptureSpecifiedMesh Thumbnails]")))
        (else
          (`KismetSystemLibrary.PrintString` (`KismetStringLibrary.Concat_StrStr` _prefix_log "没有要生成的模型！") :!label _label))))
    (:`Is Not Valid`
      (goto _label))))

(fn `CaptureAll`
  (params (Selection :type "/ThumbnailHelper/ENUM_CaptureOptions Enum" :default "NewEnumerator0") (InputIndex :type Integer :default -1))
  (bind _mats (`self.Mats`))
  (bind _defaultmesh (`self.DefaultMesh`))
  (bind _output (`|GetArrayItem` (`self.Meshs`) InputIndex))
  (bind _output_2 (`|GetArrayItem` (`self.Meshs`) 0))
  (switch `/ThumbnailHelper/ENUM_CaptureOptions` Selection
    (:`NewEnumerator0`
      ;[1 1 1] Model ONLY
      (`self.Capture Mesh Original Thumbnails`))
    (:`NewEnumerator1`
      ;[1 1 1] Material ONLY
      (`self.Capture Mat Thumbnails` (`self.Mats`)))
    (:`NewEnumerator2`
      ;[1 1 1] ALL
      (`self.Capture Mesh Original Thumbnails`)
      (for _array_element (`self.Meshs`)
        (bind _res (`self.UpdateNeedCaptureMesh` _array_element))
        (if _res
          (`self.Capture Mat Thumbnails` (`self.Mats`))
          (else
            (`self.FailLog` "Update NeedCaptureObject Failed")))))
    (:`NewEnumerator3`
      ;[1 1 1] Debug
      (bind _res_2 (`self.UpdateNeedCaptureMesh` (`self.DefaultMesh`)))
      (if _res_2
        (`self.Capture Mat Thumbnails` (`|MakeArray` (`self.DefaultMat`)))
        (else
          (`self.FailLog` "Update NeedCaptureObject Failed"))))
    (:`NewEnumerator4`
      ;[1 1 1] Specify Model Only
      (if (`KismetArrayLibrary.Array_IsValidIndex` (`self.Meshs`) InputIndex)
        (`/Engine/EditorBlueprintResources/StandardMacros.IsValid` _output
          (:`Is Valid`
            (bind _res_3 (`self.UpdateNeedCaptureMesh` _output))
            (if _res_3
              (`self.Capture SpecifiedMesh Thumbnails` (`|MakeArray` (`self.DefaultMat`)) _output)
              (else
                (`self.FailLog` "Update NeedCaptureObject Failed"))))
          (:`Is Not Valid`
            (`self.FailLog` "Mesh[index] mesh is not valid" :!label _label)))
        (else
          (goto _label))))
    (:`NewEnumerator6`
      ;[1 1 1] Specify Model Only
      (if (`KismetArrayLibrary.Array_IsValidIndex` _mats InputIndex)
        (`/Engine/EditorBlueprintResources/StandardMacros.IsValid` _defaultmesh
          (:`Is Valid`
            (bind _res_4 (`self.UpdateNeedCaptureMesh` _defaultmesh))
            (if _res_4
              (`self.Capture SpecifiedMesh Thumbnails` (`|MakeArray` (`|GetArrayItem` _mats InputIndex)) _defaultmesh)
              (else
                (`self.FailLog` "Update NeedCaptureObject Failed"))))
          (:`Is Not Valid`
            (`self.FailLog` "Default Mesh is not valid" :!label _label_2)))
        (else
          (goto _label_2))))
    (:`NewEnumerator5`
      ;[1 1 1] Specify Model Only
      (if (`KismetArrayLibrary.Array_IsValidIndex` (`self.Meshs`) 0)
        (`/Engine/EditorBlueprintResources/StandardMacros.IsValid` _output_2
          (:`Is Valid`
            (bind _res_5 (`self.UpdateNeedCaptureMesh` _output_2))
            (if _res_5
              (`KismetArrayLibrary.Array_Add` (`self.Mats`) (`self.DefaultMat`))
              (`self.Capture SpecifiedMesh Thumbnails` (`self.Mats`) _output_2)
              (else
                (`self.FailLog` "Update NeedCaptureObject Failed"))))
          (:`Is Not Valid`
            (`self.FailLog` "Mesh[index] mesh is not valid" :!label _label_3)))
        (else
          (goto _label_3))))))

(fn `CenterDefaultMesh`
  (bind _centerboundreference (`self.CenterBoundReference`))
  (bind _needcaptureobject (`self.NeedCaptureObject`))
  (bind (_min _max) (`StaticMeshComponent.GetLocalBounds` _centerboundreference))
  (bind (_min_2 _max_2) (`StaticMeshComponent.GetLocalBounds` _needcaptureobject))
  (bind _returnvalue (* (- _max_2 _min_2) 0.5))
  (bind _returnvalue_2 (* (* (`SceneComponent.K2_GetComponentScale` _centerboundreference) (- _max _min)) 0.5))
  (bind _returnvalue_3 (/ _returnvalue_2 _returnvalue))
  (`SceneComponent.SetWorldScale3D` _needcaptureobject _returnvalue_3)
  (`SceneComponent.SetWorldScale3D` (`self.CenterPointReference1`) (* (/ _returnvalue _returnvalue_2) 0.5))
  (`KismetSystemLibrary.PrintString` (`KismetStringLibrary.Concat_StrStr` (`self.Prefix-Log`) "Set Relative Transform" " \n        " "[Scale]" (`KismetStringLibrary.Concat_StrStr` "{   " (`KismetStringLibrary.Conv_DoubleToString` (.x _returnvalue_3)) "    ,    " (`KismetStringLibrary.Conv_DoubleToString` (.y _returnvalue_3)) "   ,   " (`KismetStringLibrary.Conv_DoubleToString` (.z _returnvalue_3)) "   }"))))

(fn `ExportThumbnail`
  (params (FileName :type String :default "Test"))
  (bind _returnvalue (`KismetStringLibrary.Concat_StrStr` FileName ".TGA"))
  (bind _scenecapturecomponent2d (`self.SceneCaptureComponent2D`))
  (bind _savedpath (`self.SavedPath`))
  ;[1 1 1] Create ScreenCapture2D at current Camera position
  (`SceneComponent.K2_SetRelativeTransform` (`self.SceneCaptureComponent2D`) (`SceneComponent.GetRelativeTransform` (`self.Camera`)) false false)
  ;[1 1 1] Set initial values for the ScreenCapture. Note "RT_SaveSlot" is a TextureTarget created and living inside the Editor
  (set `SceneCaptureComponent.CaptureSource` "SCS_SceneColorSceneDepth" (`self.SceneCaptureComponent2D`))
  (set `SceneCaptureComponent2D.FOVAngle` (`CameraComponent.FieldOfView` (`self.Camera`)) _scenecapturecomponent2d)
  (set `SceneCaptureComponent2D.TextureTarget` (`self.RT`) _scenecapturecomponent2d)
  ;;[1 1 1] Improves performance by not capturing every frame
  (set `SceneCaptureComponent.bCaptureEveryFrame` false _scenecapturecomponent2d)
  (set `SceneCaptureComponent.bCaptureOnMovement` false _scenecapturecomponent2d)
  (`SceneComponent.SetVisibility` (`self.CenterPointReference`) false false)
  (`SceneComponent.SetVisibility` (`self.CenterBoundReference`) false false)
  (`SceneComponent.SetVisibility` (`self.CenterPointReference1`) false false)
  ;[1 1 1] Capture camara view and export the image as binary to the SaveGames folder with name "<SAVE_SLOT>_Thumbnail"
  (`SceneCaptureComponent2D.CaptureScene` (`self.SceneCaptureComponent2D`))
  (`KismetRenderingLibrary.ExportRenderTarget` (`SceneCaptureComponent2D.TextureTarget` (`self.SceneCaptureComponent2D`)) _savedpath _returnvalue)
  (`KismetSystemLibrary.PrintString` (`KismetStringLibrary.Concat_StrStr` "一键生成缩略图工具  " "材质缩略图生成完成" (`KismetStringLibrary.Concat_StrStr` _savedpath _returnvalue)))
  (`SceneComponent.SetVisibility` (`self.CenterPointReference`) false false)
  (`SceneComponent.SetVisibility` (`self.CenterBoundReference`) false false))

(fn `FailLog`
  (params (InputStr :type String))
  (bind _prefix_log (`self.Prefix-Log`))
  (`KismetSystemLibrary.PrintString` (`KismetStringLibrary.Concat_StrStr` _prefix_log "Failed!"))
  (`KismetSystemLibrary.PrintString` (`KismetStringLibrary.Concat_StrStr` _prefix_log InputStr)))

(fn `SetupInputAssets`
  (params (Mesh :type "Array of StaticMesh Object Reference") (Mat :type "Array of MaterialInstanceConstant Object Reference"))
  (bind _meshs (`self.Meshs`))
  (bind _mats (`self.Mats`))
  (if (> (`KismetArrayLibrary.Array_Length` Mesh) 0)
    (for _array_element Mesh
      (if (not (`KismetArrayLibrary.Array_Contains` _meshs _array_element))
        (`KismetArrayLibrary.Array_Add` _meshs _array_element))))
  (if (> (`KismetArrayLibrary.Array_Length` Mat) 0)
    (for _array_element_2 Mat
      (if (not (`KismetArrayLibrary.Array_Contains` _mats _array_element_2))
        (`KismetArrayLibrary.Array_Add` _mats _array_element_2)))))

(fn `UpdateNeedCaptureMesh`
  (params (InputObject :type "StaticMesh Object Reference"))
  (returns (Res :type Boolean))
  (`/Engine/EditorBlueprintResources/StandardMacros.IsValid` InputObject
    (:`Is Valid`
      (`StaticMeshComponent.SetStaticMesh` (`self.NeedCaptureObject`) InputObject)
      (`self.CenterDefaultMesh`)
      (return true))
    (:`Is Not Valid`
      (`KismetSystemLibrary.PrintString` (`KismetStringLibrary.Concat_StrStr` (`self.Prefix-Log`) "Default Mesh is not  Valid"))
      (return false))))

(fn `UpdateSavedPath`
  (bind _rt (`self.RT`))
  (bind _returnvalue (`KismetStringLibrary.Concat_StrStr` (`KismetSystemLibrary.ConvertToAbsolutePath` (`KismetSystemLibrary.GetProjectSavedDirectory`)) "ThumbnailHelper/"))
  (bind _returnvalue_2 (`KismetStringLibrary.Concat_StrStr` (`KismetStringLibrary.Replace` (`KismetStringLibrary.Split` (`KismetStringLibrary.Replace` (`KismetSystemLibrary.ConvertToAbsolutePath` (`KismetSystemLibrary.GetSystemPath` _rt)) "/Game/") ".") (`KismetSystemLibrary.GetDisplayName` _rt)) "Saved/"))
  ;[1 1 1] ThumbnailHelper Dir
  (if (`KismetSystemLibrary.IsValid` _rt)
    (if (`BlueprintPathsLibrary.DirectoryExists` (`KismetStringLibrary.Replace` _returnvalue_2 "//" "/"))
      (set `self.SavedPath` _returnvalue_2)
      (else
        (`self.FailLog` (`KismetStringLibrary.Concat_StrStr` "Directory   ||   " "" "   Not Exists!" "      New Saved Path   is    " _returnvalue))
        (set `self.SavedPath` _returnvalue :!label _label)))
    (else
      (`self.FailLog` "RT Settings Empty!")
      (goto _label))))

(fn `UserConstructionScript`
  (`self.UpdateSavedPath`))